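; TarGame is a game-logic Blueprint that respawns the player's TervaCharacter whenever it is destroyed.
; On BeginPlay it binds to the character's OnDestroyed event.
; When that fires, it spawns a new TervaCharacter at a stored transform and has the first player controller possess it, provided that controller is a TervaController.
; A Respawn event then loops back to rebind the destruction handler, so the cycle repeats.
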(event `self.ReceiveBeginPlay`
  (bind _astervacharacter_c (cast `/Game/Blueprints/TervaCharacter` (`GameplayStatics.GetPlayerCharacter` 0) :!label _label))
  (add `self.OnDestroyed` _astervacharacter_c (delegate `OnDestroyed_Event`)))

(event `Respawn`
  (goto _label))

(event `OnDestroyed_Event`
  (bind _astervacontroller_c (cast `/Game/Blueprints/TervaController` (`GameplayStatics.GetPlayerController` 0)))
  (bind _returnvalue (`|SpawnActorFromClass` "/Game/Blueprints/TervaCharacter.TervaCharacter_C" (`self.SpawnTransfomr`) false 6.0))
  (`Controller.Possess` (`GameplayStatics.GetPlayerController` 0) _returnvalue)
  (`self.Respawn`))

(fn `UserConstructionScript`)