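; DoorLevelport is a door Blueprint that lets the player travel to another level by pressing a key while standing near it.
; Overlap events on TriggerVolume enable or disable the actor's input for the player pawn and toggle the PressDown prompt's visibility on entry and exit.
; While input is enabled, the InspectBackground action opens the level named by TargetLevel.
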(event `self.TriggerVolume.OnComponentBeginOverlap`
  (params (OtherActor :type "Actor Object Reference") (OtherComp :type "PrimitiveComponent Object Reference") (OtherBodyIndex :type Integer) (bFromSweep :type Boolean) (SweepResult :type "EngineTypes.HitResult Structure (by ref)"))
  ;[1 1 1] Toggles teleport ability and visual cues on player overlap
  (if (== OtherActor (`GameplayStatics.GetPlayerPawn` 0))
    (`self.EnableInput` (`GameplayStatics.GetPlayerController` 0))
    (`SceneComponent.ToggleVisibility` (`self.PressDown`) true :!label _label)))

(event `self.TriggerVolume.OnComponentEndOverlap`
  (params (OtherActor :type "Actor Object Reference") (OtherComp :type "PrimitiveComponent Object Reference") (OtherBodyIndex :type Integer))
  ;[1 1 1] Toggles teleport ability and visual cues on player overlap
  (if (== (`GameplayStatics.GetPlayerPawn` 0) OtherActor)
    (`self.DisableInput` (`GameplayStatics.GetPlayerController` 0))
    (goto _label)))

(event `InputAction|InspectBackground`
  (:`Pressed`
    (`GameplayStatics.OpenLevel` (`self.TargetLevel`))))

(fn `UserConstructionScript`
  (`parent.UserConstructionScript`))