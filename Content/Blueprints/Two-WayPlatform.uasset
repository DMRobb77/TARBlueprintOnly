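; Two-way platform that the player can pass up through from below or drop down through from on top.
; BottomTrigger sets the mesh to ignore the Pawn channel while the player overlaps it.
; TopTrigger enables actor input during overlap, so InspectBackground, or Down held on entry, makes the mesh passable.
; Leaving either trigger restores blocking, and the collision change applies to all pawns.
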(event `self.BottomTrigger.OnComponentBeginOverlap`
  (params (OtherActor :type "Actor Object Reference") (OtherComp :type "PrimitiveComponent Object Reference") (OtherBodyIndex :type Integer) (bFromSweep :type Boolean) (SweepResult :type "EngineTypes.HitResult Structure (by ref)"))
  (if (== OtherActor (`GameplayStatics.GetPlayerPawn` 0))
    (`PrimitiveComponent.SetCollisionResponseToChannel` (`self.PlatMesh`) "ECC_Pawn" "ECR_Ignore")))

(event `self.BottomTrigger.OnComponentEndOverlap`
  (params (OtherActor :type "Actor Object Reference") (OtherComp :type "PrimitiveComponent Object Reference") (OtherBodyIndex :type Integer))
  (if (== (`GameplayStatics.GetPlayerPawn` 0) OtherActor)
    (`PrimitiveComponent.SetCollisionResponseToChannel` (`self.PlatMesh`) "ECC_Pawn" "ECR_Block")))

(event `self.TopTrigger.OnComponentBeginOverlap`
  (params (OtherActor :type "Actor Object Reference") (OtherComp :type "PrimitiveComponent Object Reference") (OtherBodyIndex :type Integer) (bFromSweep :type Boolean) (SweepResult :type "EngineTypes.HitResult Structure (by ref)"))
  (bind _returnvalue (`GameplayStatics.GetPlayerController` 0))
  (if (== OtherActor (`GameplayStatics.GetPlayerPawn` 0))
    (`self.EnableInput` (`GameplayStatics.GetPlayerController` 0))
    (if (or (`PlayerController.IsInputKeyDown` _returnvalue "Down") (`PlayerController.IsInputKeyDown` _returnvalue "Gamepad_DPad_Down"))
      (`PrimitiveComponent.SetCollisionResponseToChannel` (`self.PlatMesh`) "ECC_Pawn" "ECR_Ignore"))))

(event `self.TopTrigger.OnComponentEndOverlap`
  (params (OtherActor :type "Actor Object Reference") (OtherComp :type "PrimitiveComponent Object Reference") (OtherBodyIndex :type Integer))
  (if (== (`GameplayStatics.GetPlayerPawn` 0) OtherActor)
    (`self.DisableInput` (`GameplayStatics.GetPlayerController` 0))
    (`PrimitiveComponent.SetCollisionResponseToChannel` (`self.PlatMesh`) "ECC_Pawn" "ECR_Block")))

(event `InputAction|InspectBackground`
  (:`Pressed`
    (`PrimitiveComponent.SetCollisionResponseToChannel` (`self.PlatMesh`) "ECC_Pawn" "ECR_Ignore")))

(fn `UserConstructionScript`)