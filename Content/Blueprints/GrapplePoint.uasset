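; Grapple point Blueprint that toggles the visibility of its GrappleLight in response to left and right trigger overlaps.
; The right trigger toggles the light on every begin and end overlap.
; The left trigger decrements Count on entry, toggling through a DoOnce, and increments it on exit.
; After a left exit, a nonzero Count toggles the light, while zero only resets the DoOnce.
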(event `self.TriggerLeft.OnComponentBeginOverlap`
  (params (OtherActor :type "Actor Object Reference") (OtherComp :type "PrimitiveComponent Object Reference") (OtherBodyIndex :type Integer) (bFromSweep :type Boolean) (SweepResult :type "EngineTypes.HitResult Structure (by ref)"))
  ;[1 1 1] Left Trigger
  (set `self.Count` (+ (`self.Count`) -1))
  (`/Engine/EditorBlueprintResources/StandardMacros.DoOnce` false :!label _label
    (:`Completed`
      (`SceneComponent.ToggleVisibility` (`self.grappleLight`) false :!label _label_2))))

(event `self.TriggerRight.OnComponentBeginOverlap`
  (params (OtherActor :type "Actor Object Reference") (OtherComp :type "PrimitiveComponent Object Reference") (OtherBodyIndex :type Integer) (bFromSweep :type Boolean) (SweepResult :type "EngineTypes.HitResult Structure (by ref)"))
  ;[1 1 1] Right Trigger
  (`SceneComponent.ToggleVisibility` (`self.grappleLight`) false :!label _label_3))

(event `self.TriggerRight.OnComponentEndOverlap`
  (params (OtherActor :type "Actor Object Reference") (OtherComp :type "PrimitiveComponent Object Reference") (OtherBodyIndex :type Integer))
  ;[1 1 1] Right Trigger
  (goto _label_3))

(event `self.TriggerLeft.OnComponentEndOverlap`
  (params (OtherActor :type "Actor Object Reference") (OtherComp :type "PrimitiveComponent Object Reference") (OtherBodyIndex :type Integer))
  (bind _count (`self.Count`))
  ;[1 1 1] Left Trigger
  (set `self.Count` (+ _count 1))
  (if (`KismetMathLibrary.Conv_IntToBool` _count)
    (goto _label_2)
    (else
      (goto _label :!via `Reset`))))

(fn `UserConstructionScript`)