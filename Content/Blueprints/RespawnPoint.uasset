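; RespawnPoint is a trigger-volume actor that responds to the player pawn entering and leaving, though no respawn logic appears in its graphs.
; Overlap begin enables the actor's input and overlap end disables it, with both toggling the PressDown prompt's visibility rather than setting it explicitly.
; Camera zoom and camera state functions return fixed defaults, and the construction script only reassigns TargetDoor to itself.
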(event `self.TriggerVolume.OnComponentBeginOverlap`
  (params (OtherActor :type "Actor Object Reference") (OtherComp :type "PrimitiveComponent Object Reference") (OtherBodyIndex :type Integer) (bFromSweep :type Boolean) (SweepResult :type "EngineTypes.HitResult Structure (by ref)"))
  (if (== OtherActor (`GameplayStatics.GetPlayerPawn` 0))
    (`self.EnableInput` (`GameplayStatics.GetPlayerController` 0))
    (`SceneComponent.ToggleVisibility` (`self.PressDown`) true :!label _label)))

(event `self.TriggerVolume.OnComponentEndOverlap`
  (params (OtherActor :type "Actor Object Reference") (OtherComp :type "PrimitiveComponent Object Reference") (OtherBodyIndex :type Integer))
  (if (== (`GameplayStatics.GetPlayerPawn` 0) OtherActor)
    (`self.DisableInput` (`GameplayStatics.GetPlayerController` 0))
    (goto _label)))

(fn `Camera Zoom Level`
  (returns (MinCameraZoom :type "Float (double-precision)"))
  (return 0.0))

(fn `Get Camera State`
  (returns (`Camera State` :type "/Game/Blueprints/Camera_States Enum"))
  (return "NewEnumerator0"))

(fn `UserConstructionScript`
  (set `self.TargetDoor` (`self.TargetDoor`)))