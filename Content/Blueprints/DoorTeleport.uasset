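; Door actor that teleports the player to a linked TargetDoor when the InspectBackground input is pressed.
; Overlapping its trigger volume enables input and toggles the PressDown prompt, and leaving disables input and toggles it back.
; Teleporting keeps the player's X and rotation while taking the target's Y and Z.
; It then snaps the TervaCharacter camera to that Y and Z, using the character's zoom level as X.
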(event `self.TriggerVolume.OnComponentBeginOverlap`
  (params (OtherActor :type "Actor Object Reference") (OtherComp :type "PrimitiveComponent Object Reference") (OtherBodyIndex :type Integer) (bFromSweep :type Boolean) (SweepResult :type "EngineTypes.HitResult Structure (by ref)"))
  ;[1 1 1] Toggles teleport ability and visual cues on player overlap
  (if (== OtherActor (`GameplayStatics.GetPlayerPawn` 0))
    (`self.EnableInput` (`GameplayStatics.GetPlayerController` 0))
    (`SceneComponent.ToggleVisibility` (`self.PressDown`) true :!label _label)))

(event `self.TriggerVolume.OnComponentEndOverlap`
  (params (OtherActor :type "Actor Object Reference") (OtherComp :type "PrimitiveComponent Object Reference") (OtherBodyIndex :type Integer))
  ;[1 1 1] Toggles teleport ability and visual cues on player overlap
  (if (== (`GameplayStatics.GetPlayerPawn` 0) OtherActor)
    (`self.DisableInput` (`GameplayStatics.GetPlayerController` 0))
    (goto _label)))

(event `InputAction|InspectBackground`
  (bind _returnvalue (`GameplayStatics.GetPlayerPawn` 0))
  (bind _targetdoor (`self.TargetDoor`))
  ;[1 1 1] Teleports the player and their camera to the specified Target Door
  (:`Pressed`
    (`/Engine/EditorBlueprintResources/StandardMacros.IsValid` _targetdoor
      (:`Is Valid`
        (`self.K2_TeleportTo` _returnvalue (`KismetMathLibrary.MakeVector` (.x (`self.K2_GetActorLocation` _returnvalue)) (.y (`self.K2_GetActorLocation` _targetdoor)) (.z (`self.K2_GetActorLocation` _targetdoor))) (`self.K2_GetActorRotation` _returnvalue))
        (bind _astervacharacter_c (cast `/Game/Blueprints/TervaCharacter` (`GameplayStatics.GetPlayerPawn` 0)))
        (bind _mincamerazoom (message `/Game/Blueprints/Camera_Interface.Camera Zoom Level` _astervacharacter_c))
        (set `self.Zoom Level` _mincamerazoom)
        (`SceneComponent.SetWorldLocation` (`/Game/Blueprints/TervaCharacter.CharCamera` _astervacharacter_c) (`KismetMathLibrary.MakeVector` (`self.Zoom Level`) (.y (`self.K2_GetActorLocation` (`self.TargetDoor`))) (.z (`self.K2_GetActorLocation` (`self.TargetDoor`)))) false)))))

(fn `Camera Zoom Level`
  (returns (MinCameraZoom :type "Float (double-precision)"))
  (return 0.0))

(fn `Get Camera State`
  (returns (`Camera State` :type "/Game/Blueprints/Camera_States Enum"))
  (return "NewEnumerator0"))

(fn `UserConstructionScript`
  (set `self.TargetDoor` (`self.TargetDoor`)))