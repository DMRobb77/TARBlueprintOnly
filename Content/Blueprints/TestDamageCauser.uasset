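; A test actor that damages the player on contact and can itself be destroyed by damage.
; On Hit, it applies fixed point damage to the first player pawn when that pawn is the other actor.
; It tracks Health from MaxHealth, clamped on any incoming damage, and at zero destroys itself and spawns an explosion emitter with random rotation.
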(event `self.ReceiveBeginPlay`
  (set `self.Health` (`self.Max Health`)))

(event `self.ReceiveHit`
  (params (MyComp :type "PrimitiveComponent Object Reference") (Other :type "Actor Object Reference") (OtherComp :type "PrimitiveComponent Object Reference") (bSelfMoved :type Boolean) (HitLocation :type "Object.Vector Structure") (HitNormal :type "Object.Vector Structure") (NormalImpulse :type "Object.Vector Structure") (Hit :type "EngineTypes.HitResult Structure (by ref)"))
  (if (== Other (`GameplayStatics.GetPlayerPawn` 0))
    (`GameplayStatics.ApplyPointDamage` Other 20.0 HitLocation Hit null self)))

(event `self.ReceiveAnyDamage`
  (params (Damage :type "Float (single-precision)") (DamageType :type "DamageType Object Reference") (InstigatedBy :type "Controller Object Reference") (DamageCauser :type "Actor Object Reference"))
  (set `self.Health` (`KismetMathLibrary.FClamp` (- (`self.Health`) Damage) 0.0 (`self.Max health`)))
  (if (<= (`self.Health`) 0.0)
    (`self.K2_DestroyActor`)
    (`GameplayStatics.SpawnEmitterAtLocation` "/Game/StarterContent/Particles/P_Explosion.P_Explosion" (`self.K2_GetActorLocation`) (`KismetMathLibrary.RandomRotator` false))))

(fn `UserConstructionScript`)