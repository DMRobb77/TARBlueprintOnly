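; Side-scrolling player character with Y-axis movement, hold-to-jump, experimental Shift sprint and clamped health.
; Tick drives a lagging camera: horizontal speed sets X zoom, facing flips the Y lead, and Y/Z stay clamped near the pawn.
; The JumpCamZ timeline varies vertical camera interp speed on jumps and ledge falls, and landing resets it.
; A child CableActor gets initial length and width, while velocity-based turning logic is disconnected.
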(event Custom|ReceiveBeginPlay_Copy
  ;[1 1 1] Cable Initializer
  (bind _ascableactor (Utilities|Casting|CastToCableActor (Variables|/Script/Engine.ChildActorComponent|GetChildActor (Variables|Default|GetCableActor))))
  (Variables|/Script/CableComponent.CableComponent|SetCableLength (Variables|/Script/CableComponent.CableActor|GetCableComponent _ascableactor) (stale _returnvalue))
  (Variables|/Script/CableComponent.CableComponent|SetCableWidth (Variables|/Script/CableComponent.CableActor|GetCableComponent _ascableactor) 5.0))

(event EventOnWalkingOffLedge
  ;[1 1 1] Smooth the camera interp speed when in the air
  (bind _caminterpspeedz (Timeline|JumpCamZ PlayFromStart)
    (:Update
      (Variables|Camera|SetCameraInterpSpeedZ _caminterpspeedz))))

(event EventOnJumped
  ;[1 1 1] Smooth the camera interp speed when in the air
  (bind _caminterpspeedz (Timeline|JumpCamZ PlayFromStart)
    (:Update
      (Variables|Camera|SetCameraInterpSpeedZ _caminterpspeedz))))

(event EventOnLanded
  (params (Hit :type Hit%20Result%20Structure%20%28by%20ref%29))
  ;[1 1 1] Smooth the camera interp speed when in the air
  (Variables|Camera|SetCameraInterpSpeedZ 2.0))

(event EventTick
  (params (DeltaSeconds :type Float%20%28single-precision%29))
  (bind _returnvalue (Game|Player|GetPlayerPawn 0))
  (bind _returnvalue_2 (Game|Player|GetPlayerPawn 0))
  (bind _camerainterpspeedxy (Variables|Camera|GetCameraInterpSpeedXY))
  (bind _camera (Variables|Default|GetCamera))
  (bind _returnvalue_3 (Transformation|GetActorLocation _returnvalue))
  (bind _returnvalue_4 (Transformation|GetActorLocation _returnvalue_2))
  (bind _returnvalue_5 (Transformation|GetWorldLocation _camera))
  (bind (_x _y _z) (Math|Vector|BreakVector _returnvalue_3))
  (bind (_x_2 _y_2 _z_2) (Math|Vector|BreakVector _returnvalue_4))
  (bind (_x_3 _y_3 _z_3) (Math|Vector|BreakVector _returnvalue_5))
  (Variables|Default|SetDelta%20Seconds DeltaSeconds)
  (Utilities|FlowControl|Sequence
    (:then_1
      (Variables|Default|SetUsable%20Velocity (Variables|/Script/Engine.MovementComponent|GetVelocity (Variables|Character|GetCharacterMovement)))
      (Variables|Camera|SetZoom%20Level (Math|Float|Lerp (Variables|Camera|GetMin%20Camera%20Zoom) (Variables|Camera|GetMax%20Camera%20Zoom) (Math|Float|Clamp(Float) (Math|Float|NormalizetoRange (Math|Float|Absolute(Float) (Math|Vector|VectorLength (* (Variables|Default|GetUsable%20Velocity) "1.000000,1.000000, 0"))) 0.0 2.5e+03))))
      (Utilities|FlowControl|Sequence
        (:then_0
          ;[1 1 1] Ensure camera starts in correct location
          (Utilities|FlowControl|DoOnce false
            (:Completed
              (Transformation|SetWorldLocation (Variables|Default|GetCamera) (Math|Vector|MakeVector (+ (Variables|Camera|GetMin%20Camera%20Zoom) _x_2) _y_2 _z_2) false))))
        (:then_1
          ;[1 1 1] Determine pawn facing direction, adjust camera Y offset accordingly
          (if (>= (Math|Float|Floor (.Yaw (Class|KismetMathLibrary|BreakRot (Transformation|GetActorRotation (Game|Player|GetPlayerPawn 0))))) 0)
            (Variables|Default|SetCameraOffsetY 144.0)
            (else
              (Variables|Default|SetCameraOffsetY -144.0))))
        (:then_2
          ;[1 1 1] Interp the current camera location to the desired location, creating camera "lag"
          (Transformation|SetWorldLocation (Variables|Default|GetCamera) (Math|Vector|MakeVector (Math|Interpolation|FInterpTo _x_3 (.X (Math|Vector|BreakVector (+ (+ (+ (Math|Vector|ClampVectorSize (* (Variables|Default|GetUsable%20Velocity) "0,0.250000,0.125000") -8e+01 8e+01) (Math|Vector|MakeVector 0.0 (Variables|Default|GetCameraOffsetY) 96.0)) (Transformation|GetActorLocation (Game|Player|GetPlayerPawn 0))) (Math|Vector|MakeVector (Variables|Camera|GetZoom%20Level) 0.0 0.0)))) (Variables|Default|GetDelta%20Seconds) _camerainterpspeedxy) (Math|Float|Clamp(Float) (Math|Interpolation|FInterpTo _y_3 (.Y (Math|Vector|BreakVector (+ (+ (+ (Math|Vector|ClampVectorSize (* (Variables|Default|GetUsable%20Velocity) "0,0.250000,0.125000") -8e+01 8e+01) (Math|Vector|MakeVector 0.0 (Variables|Default|GetCameraOffsetY) 96.0)) (Transformation|GetActorLocation (Game|Player|GetPlayerPawn 0))) (Math|Vector|MakeVector (Variables|Camera|GetZoom%20Level) 0.0 0.0)))) (Variables|Default|GetDelta%20Seconds) _camerainterpspeedxy) (- _y (Variables|Camera|GetCameraConstraint)) (+ _y (Variables|Camera|GetCameraConstraint))) (Math|Float|Clamp(Float) (Math|Interpolation|FInterpTo _z_3 (.Z (Math|Vector|BreakVector (+ (+ (+ (Math|Vector|ClampVectorSize (* (Variables|Default|GetUsable%20Velocity) "0,0.250000,0.125000") -8e+01 8e+01) (Math|Vector|MakeVector 0.0 (Variables|Default|GetCameraOffsetY) 96.0)) (Transformation|GetActorLocation (Game|Player|GetPlayerPawn 0))) (Math|Vector|MakeVector (Variables|Camera|GetZoom%20Level) 0.0 0.0)))) (Variables|Default|GetDelta%20Seconds) (Variables|Camera|GetCameraInterpSpeedZ)) (- _z (Variables|Camera|GetCameraConstraint)) (+ _z (Variables|Camera|GetCameraConstraint)))) false))))))

(event EventAnyDamage
  (params (Damage :type Float%20%28single-precision%29) (DamageType :type Damage%20Type%20Object%20Reference) (InstigatedBy :type Controller%20Object%20Reference) (DamageCauser :type Actor%20Object%20Reference))
  ;[1 1 1] When damaged reduce health
  (Variables|Default|SetHealth (Math|Float|Clamp(Float) (- (Variables|Default|GetHealth) Damage) 0.0 (Variables|Default|GetMax%20health))))

(event Input|ActionEvents|InputActionJump
  ;[1 1 1] Jump Affected by Time Button Held
  (:Pressed
    (if (Character|CanJump)
      (Character|Jump)))
  (:Released
    (Character|StopJumping)))

(event Input|AxisEvents|InputAxisMoveRight
  (params (AxisValue :type Float%20%28single-precision%29))
  ;[1 1 1] Movement inputs
  (Pawn|Input|AddMovementInput "0,1.000000, 0" AxisValue false))

(event Input|KeyboardEvents|LeftShift
  (bind _charactermovement (Variables|Character|GetCharacterMovement))
  (bind _charactermovement_2 (Variables|Character|GetCharacterMovement))
  ;[1 1 1] Running (Experimental
  (:Pressed
    (Variables|Default|SetDefaultWalkSpeed (Variables|/Script/Engine.CharacterMovementComponent|GetMaxWalkSpeed _charactermovement_2))
    (Variables|Default|SetDefaultDecel (Variables|/Script/Engine.CharacterMovementComponent|GetBrakingDecelerationWalking _charactermovement_2))
    (Variables|/Script/Engine.CharacterMovementComponent|SetMaxWalkSpeed _charactermovement (+ (Variables|Default|GetDefaultWalkSpeed) (Variables|Default|GetSprintSpeedIncrease))))
  (:Released
    (Variables|/Script/Engine.CharacterMovementComponent|SetMaxWalkSpeed _charactermovement (Variables|Default|GetDefaultWalkSpeed))))

(fn ConstructionScript)

(fn CameraZoomLevel
  (return (Variables|Camera|GetMin%20Camera%20Zoom)))

(fn GetCameraState
  (return "NewEnumerator0"))

(fn GetPlayerHealth
  (return (Variables|Default|GetHealth) (Variables|Default|GetMax%20Health)))